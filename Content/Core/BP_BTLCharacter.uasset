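; BP_BTLCharacter is a character Blueprint that adds debug shortcuts and death handling on top of its health and inventory components.
; Debug keys H, G and B send a negative "Debug hurt" damage instance to health, create and give a pistol, and add bullet ammo.
; When the health component reports a kill, the menu level opens.
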(event OnKilled(HealthComponent)
  (params (DamageInstance :type Damage%20Instance%20Structure%20%28by%20ref%29))
  (Game|OpenLevel(byObjectReference) "/Game/Levels/LVL_Menu.LVL_Menu"))

(event Input|KeyboardEvents|DebugKeyH
  (params (Key :type Key%20Structure :default "None") (ActionValue :type Input%20Action%20Value%20Structure))
  (:Pressed
    (Class|HealthComponent|ReceiveDamageInstance (Class|BTLPlayerCharacter|GetHealthComponent) (Utilities|Struct|MakeDamageInstance -1e+01 0 "Debug hurt"))))

(event Input|KeyboardEvents|DebugKeyG
  (params (Key :type Key%20Structure :default "None") (ActionValue :type Input%20Action%20Value%20Structure))
  (:Pressed
    (bind _returnvalue (Class|Weapon|CreateWeapon self "/Game/Weapons/Pistol/WPN_Pistol.WPN_Pistol"))
    (Class|InventoryComponent|GiveWeapon (Variables|Default|GetInventoryComponent) _returnvalue)))

(event Input|KeyboardEvents|DebugKeyB
  (params (Key :type Key%20Structure :default "None") (ActionValue :type Input%20Action%20Value%20Structure))
  (:Pressed
    (Class|InventoryComponent|GiveAmmo (Variables|Default|GetInventoryComponent) "Bullet" 50)))

(fn ConstructionScript)