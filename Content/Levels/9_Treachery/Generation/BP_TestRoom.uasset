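; BP_TestRoom is a generated dynamic mesh actor that builds a hollow cylindrical test room with Geometry Script on each mesh rebuild.
; Generate extrudes a circular polygon in a pooled mesh, appends it to the target, then subtracts a slightly shrunken copy to leave a closed shell.
; The shell is then uniformly remeshed, with normals and UVs recomputed and the UVs scaled down.
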(event Events|EventOnRebuildGeneratedMesh
  (params (TargetMesh :type Dynamic%20Mesh%20Object%20Reference))
  (CallFunction|Generate TargetMesh))

(fn ConstructionScript)

(fn Generate
  (params (Mesh :type Dynamic%20Mesh%20Object%20Reference))
  (bind _returnvalue (GeometryScript|Utility|CreateDynamicMeshPool))
  (LocalVariables|SetMeshPool _returnvalue)
  (bind _returnvalue_2 (Class|GeometryScriptLibraryPolyPathFunctions|CreateCirclePath3D :Radius 3e+02 :NumPoints 20))
  (bind _returnvalue_3 (Class|DynamicMeshPool|RequestMesh (LocalVariables|GetMeshPool)))
  (bind _returnvalue_4 (Class|GeometryScriptLibraryMeshPrimitiveFunctions|AppendSimpleExtrudePolygon :TargetMesh _returnvalue_3 :PolygonVertices (Class|GeometryScriptLibraryPolyPathFunctions|ToArrayOfVector2D(GeometryScriptPolyPath) _returnvalue_2) :Height 5e+02 :HeightSteps 6 :Origin "Center" :Debug 0))
  (bind _returnvalue_5 (GeometryScript|MeshEdits|AppendMesh :TargetMesh Mesh :AppendMesh _returnvalue_4 :AppendOptions "(CombineMode=EnableAllMatching)" :Debug 0))
  (bind _returnvalue_6 (Class|GeometryScriptLibraryMeshTransformFunctions|ScaleMesh _returnvalue_4 "0.900000,0.900000,0.900000" "0.000000,0.000000,0.000000" true 0))
  (bind _returnvalue_7 (GeometryScript|Booleans|ApplyMeshBoolean :TargetMesh _returnvalue_5 :ToolMesh _returnvalue_6 :Operation "Subtract" :Debug 0))
  (bind _returnvalue_8 (Class|GeometryScriptLibraryRemeshingFunctions|ApplyUniformRemesh :TargetMesh _returnvalue_7 :RemeshOptions (Utilities|Struct|MakeGeometryScriptRemeshOptions false true "Uniform" 0.25 "Free" "Free" "Free" true true true true true false 20 true) :Debug 0))
  (bind _returnvalue_9 (GeometryScript|Normals|RecomputeNormals :TargetMesh _returnvalue_8 :Debug 0))
  (bind _returnvalue_10 (Class|GeometryScriptLibraryMeshUVFunctions|RecomputeMeshUVs :TargetMesh _returnvalue_9 :Options (Utilities|Struct|MakeGeometryScriptRecomputeUVsOptions "SpectralConformal" "UVIslands" "(NormalSmoothingRounds=0,NormalSmoothingAlpha=0.250000)" (Utilities|Struct|MakeGeometryScriptSpectralConformalUVOptions false) "(bDefaultLayer=True,ExtendedLayerIndex=0)" true) :Debug 0))
  (GeometryScript|UVs|ScaleMeshUVs :TargetMesh _returnvalue_10 :Scale "(X=0.200000,Y=0.200000)" :Debug 0))