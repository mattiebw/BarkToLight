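; BP_TestCube is a Geometry Script generated-mesh actor in the Treachery level's generation folder that builds a box sized by BoxX, BoxY and BoxZ.
; On each mesh rebuild it creates a box in a pooled temporary mesh and appends it to the target mesh.
; It then recomputes normals and UVs, scales the UVs down and generates collision on the dynamic mesh component from the result.
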(event Events|EventOnRebuildGeneratedMesh
  (params (TargetMesh :type Dynamic%20Mesh%20Object%20Reference))
  (bind _returnvalue (GeometryScript|Utility|CreateDynamicMeshPool))
  (bind _returnvalue_2 (Class|DynamicMeshPool|RequestMesh _returnvalue))
  (bind _returnvalue_3 (Class|GeometryScriptLibraryMeshPrimitiveFunctions|AppendBox :TargetMesh _returnvalue_2 :DimensionX (Variables|Default|GetBox%20X) :DimensionY (Variables|Default|GetBox%20Y) :DimensionZ (Variables|Default|GetBox%20Z) :Debug 0))
  (bind _returnvalue_4 (GeometryScript|MeshEdits|AppendMesh :TargetMesh TargetMesh :AppendMesh _returnvalue_3 :AppendOptions "(CombineMode=EnableAllMatching)" :Debug 0))
  (bind _returnvalue_5 (GeometryScript|Normals|RecomputeNormals _returnvalue_4 (Utilities|Struct|MakeGeometryScriptCalculateNormalsOptions true true) false 0))
  (bind _returnvalue_6 (Class|GeometryScriptLibraryMeshUVFunctions|RecomputeMeshUVs :TargetMesh _returnvalue_5 :Debug 0))
  (bind _returnvalue_7 (GeometryScript|UVs|ScaleMeshUVs :TargetMesh _returnvalue_6 :Scale "(X=0.200000,Y=0.200000)" :Debug 0))
  (Class|GeometryScriptLibraryCollisionFunctions|SetDynamicMeshCollisionfromMesh :FromDynamicMesh _returnvalue_7 :ToDynamicMeshComponent (Class|DynamicMeshActor|GetDynamicMeshComponent) :Debug 0))

(fn ConstructionScript)