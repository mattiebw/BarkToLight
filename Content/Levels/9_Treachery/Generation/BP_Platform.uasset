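; BP_Platform is a generated-mesh actor that procedurally builds a rock-like platform for the Treachery level.
; On rebuild it appends a box sized by PlatformSize, tessellates it, and selects vertices with a downward-facing plane near the base.
; Seeded Perlin noise displaces that selection along normals to roughen the underside, then normals and UVs are recomputed and UVs scaled.
; Normal-angle selection and selection-combining nodes are left unconnected.
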(event Events|EventOnRebuildGeneratedMesh
  (params (TargetMesh :type Dynamic%20Mesh%20Object%20Reference))
  (bind _platform_size (Variables|Default|GetPlatform%20Size))
  (bind _returnvalue (Class|GeometryScriptLibraryMeshPrimitiveFunctions|AppendBox :TargetMesh TargetMesh :PrimitiveOptions (Utilities|Struct|MakeGeometryScriptPrimitiveOptions "PerQuad" false "Uniform") :DimensionX (.x _platform_size) :DimensionY (.y _platform_size) :DimensionZ (.z _platform_size) :Debug 0))
  (bind _returnvalue_2 (Class|GeometryScriptLibraryMeshSubdivideFunctions|ApplyUniformTessellation _returnvalue 3 0))
  (bind (_selection _returnvalue_3) (Class|GeometryScriptLibraryMeshSelectionFunctions|SelectMeshElementswithPlane _returnvalue_2 "0.000000,0.000000,1.000000" "0.000000,0.000000,-1.000000" "Vertices" false))
  (bind _returnvalue_4 (Class|GeometryScriptLibraryMeshDeformFunctions|ApplyPerlinNoisetoMesh _returnvalue_3 _selection (Utilities|Struct|MakeGeometryScriptPerlinNoiseOptions (Utilities|Struct|MakeGeometryScriptPerlinNoiseLayerOptions 1e+02 0.25 "0.000000,0.000000,0.000000" (Variables|Default|GetSeed)) true "FullMeshSelection") 0))
  (bind _returnvalue_5 (GeometryScript|Normals|RecomputeNormals :TargetMesh _returnvalue_4 :Debug 0))
  (bind _returnvalue_6 (Class|GeometryScriptLibraryMeshUVFunctions|RecomputeMeshUVs :TargetMesh _returnvalue_5 :Debug 0))
  (GeometryScript|UVs|ScaleMeshUVs :TargetMesh _returnvalue_6 :Scale "(X=0.100000,Y=0.100000)" :Debug 0))

(fn ConstructionScript)