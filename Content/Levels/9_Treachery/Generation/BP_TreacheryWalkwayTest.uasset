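; BP_TreacheryWalkwayTest is a generated dynamic mesh test actor for a walkway in the Treachery level.
; On mesh rebuild it samples its spline into transforms, roughly one per 100 units of length, placed by the spline's relative transform.
; A fixed square profile is swept along those frames with Geometry Script, raised on Z by half of a Radius variable.
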(event Events|EventOnRebuildGeneratedMesh
  (params (TargetMesh :type Dynamic%20Mesh%20Object%20Reference))
  (bind _spline (Variables|Default|GetSpline))
  (bind _frames (Class|GeometryScriptLibraryPolyPathFunctions|SampleSplinetoTransforms _spline (Utilities|Struct|MakeGeometryScriptSplineSamplingOptions (Math|Float|Truncate (* (Spline|GetSplineLength _spline) 0.01)) 1.0 "UniformDistance" "Local" "FullSpline" 0.0 1.0) (Transformation|GetRelativeTransform _spline) true))
  (Class|GeometryScriptLibraryMeshPrimitiveFunctions|AppendSweepPolygon :TargetMesh TargetMesh :Transform (Math|Transform|MakeTransform (Math|Vector|MakeVector 0.0 0.0 (/ (Variables|Default|GetRadius) 2.0))) :PolygonVertices (Utilities|Array|MakeArray "(X=-50.000000,Y=-50.000000)" "(X=50.000000,Y=-50.000000)" "(X=50.000000,Y=50.000000)" "(X=-50.000000,Y=50.000000)") :SweepPath _frames :Debug 0))

(fn ConstructionScript)